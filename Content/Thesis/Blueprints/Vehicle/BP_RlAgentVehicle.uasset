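; Player-drivable Chaos vehicle, named as an RL agent, that triggers screen-capture data gathering as it is driven.
; Enhanced Input accumulates clamped throttle and steering, resetting them on release, and passes brake input straight to the movement component.
; The first control input starts gathering on the level's BP_ScreenCapture, guarded by a one-time flag.
; Mesh overlaps print wall hits and quit the game at BP_Goal; EnableController enables player input.
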(event OnComponentBeginOverlap(ChaosVehicleMesh)
  (params (OverlappedComponent :type Primitive%20Component%20Object%20Reference) (OtherActor :type Actor%20Object%20Reference) (OtherComp :type Primitive%20Component%20Object%20Reference) (OtherBodyIndex :type Integer) (bFromSweep :type Boolean) (SweepResult :type Hit%20Result%20Structure%20%28by%20ref%29))
  (Utilities|Casting|CastToBP_WallMaster OtherActor
    (:then
      (Utilities|FlowControl|Sequence
        (:then_0
          (Development|PrintString "Hit Wall!" true true "(R=0.221023,G=0.279967,B=1.000000,A=1.000000)" 4.0))
        (:then_1
          (Utilities|Casting|CastToBP_Goal OtherActor :!label _label)
          (Game|QuitGame 0 "Quit" false))))
    (:CastFailed
      (goto _label))))

(event Custom|EnableController
  (bind _asvehicle_player_controller (Utilities|Casting|CastToVehiclePlayerController (Game|GetPlayerController 0)))
  (Input|EnableInput _asvehicle_player_controller))

(event Input|EnhancedActionEvents|EnhancedInputActionIA_Break
  (params (ActionValue :type Float%20%28double-precision%29) (ElapsedSeconds :type Float%20%28double-precision%29) (TriggeredSeconds :type Float%20%28double-precision%29) (InputAction :type Input%20Action%20Object%20Reference :default "/Game/Thesis/Blueprints/Input/Actions/IA_Break.IA_Break"))
  (bind _chaosvehiclemovementcomponent (Variables|Default|GetChaosVehicleMovementComponent))
  (:Triggered
    (Class|ChaosVehicleMovementComponent|SetBrakeInput _chaosvehiclemovementcomponent ActionValue)
    (Utilities|EnableDataGathering))
  (:Completed
    (Class|ChaosVehicleMovementComponent|SetBrakeInput _chaosvehiclemovementcomponent 0.0)))

(event Input|EnhancedActionEvents|EnhancedInputActionIA_Throttle
  (params (ActionValue :type Float%20%28double-precision%29) (ElapsedSeconds :type Float%20%28double-precision%29) (TriggeredSeconds :type Float%20%28double-precision%29) (InputAction :type Input%20Action%20Object%20Reference :default "/Game/Thesis/Blueprints/Input/Actions/IA_Throttle.IA_Throttle"))
  (:Triggered
    (bind _output_get (Variables|Default|SetCurrentThrottle (Math|Float|Clamp(Float) (+ (* ActionValue (Variables|Default|GetthrottleIncrease)) (Variables|Default|GetCurrentThrottle))) :!label _label))
    (Class|ChaosVehicleMovementComponent|SetThrottleInput (Variables|Default|GetChaosVehicleMovementComponent) _output_get)
    (Development|PrintString (Utilities|String|Append "current throttle" (Utilities|String|ToString(Float) (Variables|Default|GetCurrentThrottle))))
    (Utilities|EnableDataGathering :!label _label_2))
  (:Ongoing
    (goto _label))
  (:Completed
    (bind _output_get_2 (Variables|Default|SetCurrentThrottle 0.0))
    (Class|ChaosVehicleMovementComponent|SetThrottleInput (Variables|Default|GetChaosVehicleMovementComponent) _output_get_2)
    (goto _label_2)))

(event Input|EnhancedActionEvents|EnhancedInputActionIA_Steering
  (params (ActionValue :type Float%20%28double-precision%29) (ElapsedSeconds :type Float%20%28double-precision%29) (TriggeredSeconds :type Float%20%28double-precision%29) (InputAction :type Input%20Action%20Object%20Reference :default "/Game/Thesis/Blueprints/Input/Actions/IA_Steering.IA_Steering"))
  (:Triggered
    (bind _output_get (Variables|Default|SetcurrentSteer (Math|Float|Clamp(Float) (+ (* ActionValue (Variables|Default|GetsteeringIncrease)) (Variables|Default|GetcurrentSteer)) -1.0) :!label _label))
    (Class|ChaosVehicleMovementComponent|SetSteeringInput (Variables|Default|GetChaosVehicleMovementComponent) _output_get)
    (Utilities|EnableDataGathering))
  (:Ongoing
    (goto _label))
  (:Completed
    (bind _output_get_2 (Variables|Default|SetcurrentSteer 0.0))
    (Class|ChaosVehicleMovementComponent|SetSteeringInput (Variables|Default|GetChaosVehicleMovementComponent) _output_get_2)))

(event EventBeginPlay
  (|CallParentFunction)
  (bind _returnvalue (Actor|GetActorOfClass "/Game/Thesis/Blueprints/ScreenCapture/BP_ScreenCapture.BP_ScreenCapture_C"))
  (Variables|Default|SetScreenCapture _returnvalue))

(event Collision|EventActorBeginOverlap
  (params (OtherActor :type Actor%20Object%20Reference)))

(event EventTick
  (params (DeltaSeconds :type Float%20%28single-precision%29)))

(fn ConstructionScript)