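; BP_ScreenCapture is an actor that rides on the reinforcement learning vehicle, BP_RlAgentVehicle, apparently as its screen-capture viewpoint.
; On BeginPlay it finds the vehicle, snaps and attaches to it, then teleports to a fixed offset along world X and Z.
; Tick is empty, older Camera-socket positioning nodes are disconnected, and GetVehicleReference is a simple lookup helper that the event graph does not call.
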(event EventBeginPlay
  (bind _returnvalue (Transformation|GetActorTransform))
  (bind (_location _rotation _scale) (Math|Transform|BreakTransform _returnvalue))
  (bind (_x _y _z) (Class|KismetMathLibrary|BreakVector3f _location))
  (bind _returnvalue_2 (Actor|GetActorOfClass "/Game/Thesis/Blueprints/Vehicle/BP_RlAgentVehicle.BP_RlAgentVehicle_C"))
  (Utilities|IsValid _returnvalue_2
    (:Is%20Valid
      (bind _output_get (Variables|Default|SetRLAgent _returnvalue_2))
      (Transformation|AttachActorToActor _output_get "" "SnapToTarget" "SnapToTarget" "KeepWorld" false)
      (Transformation|SetActorTransform (Math|Transform|MakeTransform (Math|Vector|MakeVector (+ _x 1e+02) _y (+ _z 5e+01)) _rotation _scale) false true))))

(event Collision|EventActorBeginOverlap
  (params (OtherActor :type Actor%20Object%20Reference)))

(event EventTick
  (params (DeltaSeconds :type Float%20%28single-precision%29)))

(fn ConstructionScript)

(fn GetVehicleReference
  (bind _returnvalue (Actor|GetActorOfClass "/Game/Thesis/Blueprints/Vehicle/BP_RlAgentVehicle.BP_RlAgentVehicle_C"))
  (return _returnvalue))