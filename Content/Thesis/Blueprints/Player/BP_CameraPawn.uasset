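; BP_CameraPawn is a camera pawn that rides on the level's BP_ScreenCapture actor.
; On BeginPlay it finds that actor by class and attaches to it, snapping location and rotation while keeping relative scale.
; An unconnected leftover chain would instead attach it to BP_RlAgentVehicle and teleport it by a fixed offset, but it never runs.
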(event EventBeginPlay
  (bind _returnvalue (Actor|GetActorOfClass "/Game/Thesis/Blueprints/ScreenCapture/BP_ScreenCapture.BP_ScreenCapture_C"))
  (Transformation|AttachActorToActor _returnvalue "None" "SnapToTarget" "SnapToTarget" "KeepRelative" false))

(event Collision|EventActorBeginOverlap
  (params (OtherActor :type Actor%20Object%20Reference)))

(event EventTick
  (params (DeltaSeconds :type Float%20%28single-precision%29)))

(fn ConstructionScript)